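; HUD for the vehicle template that draws the speed and gear readouts of the possessed VehicleBlueprint.
; DrawHUD shows them only while IsInCar is false, using display strings read from the pawn.
; Text position and size scale from a 1280x720 reference resolution.
; The gear text switches between the pawn's reverse and normal colors based on InReverseGear.
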(event `self.ReceiveDrawHUD`
  (params (SizeX :type Integer) (SizeY :type Integer))
  (bind _hudyratio (`self.HUDYRatio`))
  (bind _hudyratio_2 (`self.HUDYRatio`))
  ;[1 1 1] Calculate ratio from 720p
  (bind _asvehicle_blueprint (cast `/Game/BP_CODE/VehicleAdvBP/Blueprints/VehicleBlueprint` (`self.GetOwningPawn`)))
  (if (not (`/Game/BP_CODE/VehicleAdvBP/Blueprints/VehicleBlueprint.IsInCar` _asvehicle_blueprint))
    (`|ExecutionSequence`
      (:`then_0`
        (set `self.HUDXRatio` (/ (`KismetMathLibrary.Conv_IntToDouble` SizeX) 1280.0)))
      (:`then_1`
        (set `self.HUDYRatio` (/ (`KismetMathLibrary.Conv_IntToDouble` SizeY) 720.0)))
      (:`then_2`
        ;[1 1 1] Print vehicle speed
        (bind _asvehicle_blueprint_2 (cast `/Game/BP_CODE/VehicleAdvBP/Blueprints/VehicleBlueprint` (`self.GetOwningPawn`)))
        (`self.DrawText` (`/Game/BP_CODE/VehicleAdvBP/Blueprints/VehicleBlueprint.Speed Display String` _asvehicle_blueprint_2) (struct :`R` 1.0 :`G` 1.0 :`B` 1.0 :`A` 1.0) (* 805.0 (`self.HUDXRatio`)) (* 455.0 _hudyratio_2) "/Engine/EngineFonts/RobotoDistanceField.RobotoDistanceField" (* 1.4 _hudyratio_2))
        ;[1 1 1] Print vehicle gear
        (bind _asvehicle_blueprint_3 (cast `/Game/BP_CODE/VehicleAdvBP/Blueprints/VehicleBlueprint` (`self.GetOwningPawn`)))
        (`self.DrawText` (`/Game/BP_CODE/VehicleAdvBP/Blueprints/VehicleBlueprint.Gear Display String` _asvehicle_blueprint_3) (`KismetMathLibrary.SelectColor` (`/Game/BP_CODE/VehicleAdvBP/Blueprints/VehicleBlueprint.GearDisplayReverseColor` _asvehicle_blueprint_3) (`/Game/BP_CODE/VehicleAdvBP/Blueprints/VehicleBlueprint.GearDisplayColor` _asvehicle_blueprint_3) (`/Game/BP_CODE/VehicleAdvBP/Blueprints/VehicleBlueprint.InReverseGear` _asvehicle_blueprint_3)) (* 805.0 (`self.HUDXRatio`)) (* 500.0 _hudyratio) "/Engine/EngineFonts/RobotoDistanceField.RobotoDistanceField" (* 1.4 _hudyratio)) ; If True display Current Gear
      ))))

(fn `UserConstructionScript`)